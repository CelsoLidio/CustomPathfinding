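; BP_GridMapping is a grid mapping Blueprint that configures its Grid object and can preview it with debug drawing.
; The construction script copies the debug flag, ground and obstacle channels, and tile size onto Grid.
; It then calls Grid's DrawGrid in debug mode or flushes persistent debug lines otherwise, while BeginPlay does nothing.
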(event `self.ReceiveBeginPlay`)

(fn `UserConstructionScript`
  (bind _output_get (set `GridComponent.isDebugMode` (`self.DebugMode`) (`self.Grid`)))
  (`self.DefaultsGrid`)
  (if _output_get
    (`GridComponent.DrawGrid` (`self.Grid`))
    (else
      (`KismetSystemLibrary.FlushPersistentDebugLines`))))